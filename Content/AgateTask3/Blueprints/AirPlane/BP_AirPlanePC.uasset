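; Player airplane Character that moves from the Up and Right input axes, stored together in a 2D InputAxis vector.
; Each Tick, DirectMovement stops movement immediately when input is zero, otherwise adds movement input along forward (X) and right (Y) vectors.
; GetWorldDirection feeds control yaw into rotator roll with zero pitch and yaw, so forward stays world X while right tilts with that angle.
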(event EventTick
  (params (DeltaSeconds :type Float%20%28single-precision%29))
  (CallFunction|DirectMovement (Variables|Default|GetInput%20Axis)))

(event Input|AxisEvents|InputAxisUp
  (params (AxisValue :type Float%20%28single-precision%29))
  (Class|KismetMathLibrary|Set2D (Variables|Default|GetInput%20Axis) AxisValue (stale Input|AxisEvents|InputAxisRight AxisValue)))

(event Input|AxisEvents|InputAxisRight
  (params (AxisValue :type Float%20%28single-precision%29))
  (Class|KismetMathLibrary|Set2D (Variables|Default|GetInput%20Axis) (stale Input|AxisEvents|InputAxisUp AxisValue) AxisValue))

(fn ConstructionScript)

(fn DirectMovement
  (params (Input%20Axis :type Vector%202D%20Structure))
  (bind (_forward_vector _right_vector) (CallFunction|GetWorldDirection))
  (bind (_x _y) (Math|Vector2D|BreakVector2D Input%20Axis))
  (Utilities|FlowControl|Sequence
    (:then_0
      (if (Class|KismetMathLibrary|IsZero2D Input%20Axis)
        (Components|Movement|StopMovementImmediately (Variables|Character|GetCharacterMovement))))
    (:then_1
      (if (!= _x 0.0)
        (Pawn|Input|AddMovementInput _forward_vector _x false)))
    (:then_2
      (if (!= _y 0.0)
        (Pawn|Input|AddMovementInput _right_vector _y false)))
    (:then_3
      (return))))

(fn GetWorldDirection
  (bind _returnvalue (Pawn|GetControlRotation :!class /Script/Engine.Pawn))
  (bind _yaw (Math|Rotator|BreakRotator _returnvalue))
  (bind _returnvalue_2 (Math|Rotator|MakeRotator _yaw 0.0 0.0))
  (return (Math|Vector|GetForwardVector _returnvalue_2) (Math|Vector|GetRightVector _returnvalue_2)))